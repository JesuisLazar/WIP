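; Simple prototype AI enemy that chases characters, attacks them in melee and can be killed.
; A looping timer sphere-traces for a nearby target to follow with AIMoveTo, wandering to random reachable points otherwise.
; Overlapping the Sphere component starts repeating montage attacks that apply damage until overlap ends.
; AnyDamage reduces health and spawns blood or, at zero, stops the AI and multicasts a ragdoll that later shrinks and is destroyed.
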(event `self.ReceiveBeginPlay`
  ;[1 1 1] Begin Play
  (`KismetSystemLibrary.Delay` 0.2)
  (`KismetSystemLibrary.K2_SetTimer` null "CheckForPlayerInRadius" 1.0 true))

(event `self.Sphere.OnComponentBeginOverlap`
  (params (OverlappedComponent :type "PrimitiveComponent Object Reference") (OtherActor :type "Actor Object Reference") (OtherComp :type "PrimitiveComponent Object Reference") (OtherBodyIndex :type Integer) (bFromSweep :type Boolean) (SweepResult :type "HitResult Structure (by ref)"))
  ;[1 1 1] Damage Player (overlap with the sphere)
  (cast `/Game/TSS_Game/Blueprints/System/BP_CharacterBase` OtherActor)
  (`self.AttackMontageMulticast`))

(event `CheckForPlayerInRadius`
  (bind _returnvalue (`self.K2_GetActorLocation`))
  ;[1 1 1] Move to nearest Player
  (bind (_outhit _returnvalue_2) (`KismetSystemLibrary.SphereTraceSingleForObjects` _returnvalue (- _returnvalue (0.0 0.0 50.0)) 800.0 (`self.ObjectType`)))
  (if _returnvalue_2
    (if (not (`self.isDead`))
      (`self.MoveToPlayer` (`.HitActor` (`GameplayStatics.BreakHitResult` _outhit))))
    (else
      ;;[1 1 1] Random Location if no Player has been detected
      (`AITask_MoveTo.AIMoveTo` (`AIBlueprintHelperLibrary.GetAIController` self) (`NavigationSystemV1.K2_GetRandomReachablePointInRadius` (`self.K2_GetActorLocation`) 500.0 null null) null 10.0 "Default" "Default" true false))))

(event `AttackMontageMulticast`
  ;[1 1 1] Attack montage
  (`/Engine/EditorBlueprintResources/StandardMacros.DoOnce` false :!label _label
    (:`Completed`
      (`KismetSystemLibrary.K2_SetTimer` null "AttackMontageMulticast" 1.0 true)
      (`AnimInstance.Montage_Play` (`SkeletalMeshComponent.GetAnimInstance` (`self.Mesh`)) "/Game/TSS_Game/Character/AnimStarterPack/ThirdPersonClimbLoop_Montage.ThirdPersonClimbLoop_Montage" 1.5 "MontageLength" 0.0 true)
      (`GameplayStatics.ApplyDamage` (stale `self.Sphere.OnComponentBeginOverlap` OtherActor) 0.1 null self)
      (`KismetSystemLibrary.RetriggerableDelay` 0.2)
      (goto _label :!via `Reset`))))

(event `self.Sphere.OnComponentEndOverlap`
  (params (OverlappedComponent :type "PrimitiveComponent Object Reference") (OtherActor :type "Actor Object Reference") (OtherComp :type "PrimitiveComponent Object Reference") (OtherBodyIndex :type Integer))
  ;[1 1 1] Damage Player (overlap with the sphere)
  (cast `/Game/TSS_Game/Blueprints/System/BP_CharacterBase` OtherActor)
  (`KismetSystemLibrary.K2_ClearTimer` null "AttackMontageMulticast"))

(event `EnemyDeadMulticast`
  (bind _capsulecomponent (`self.CapsuleComponent`))
  ;[1 1 1] Happens on all clients
  (`PrimitiveComponent.SetCollisionResponseToChannel` _capsulecomponent "ECC_Pawn" "ECR_Ignore")
  (`PrimitiveComponent.SetCollisionResponseToChannel` _capsulecomponent "ECC_Visibility" "ECR_Ignore")
  (`PrimitiveComponent.SetCollisionEnabled` (`self.Sphere`) "NoCollision")
  (`PrimitiveComponent.SetSimulatePhysics` (`self.Mesh`) true)
  (`KismetSystemLibrary.Delay` 10.0)
  (bind (_direction _duration) (`Timeline|Timeline_0` :!via `PlayFromStart`)
    (:`Update`
      (`SceneComponent.SetWorldScale3D` (`self.Mesh`) (`KismetMathLibrary.VLerp` (1.0 1.0 1.0) (0.0 0.0 0.0) _duration)))
    (:`Finished`
      (`self.K2_DestroyActor`))))

(event `MoveToPlayer`
  (params (GoalActor :type "Actor Object Reference"))
  ;[1 1 1] Move to nearest Player
  (if (not (`self.isDead`))
    (`AITask_MoveTo.AIMoveTo` (`AIBlueprintHelperLibrary.GetAIController` self) (0.0 0.0 0.0) GoalActor 10.0 "Default" "Default" true false)))

(event `self.ReceiveAnyDamage`
  (params (Damage :type "Float (single-precision)") (DamageType :type "DamageType Object Reference") (InstigatedBy :type "Controller Object Reference") (DamageCauser :type "Actor Object Reference"))
  (bind _charactermovement (`self.CharacterMovement`))
  (bind _playerstate (`Controller.PlayerState` InstigatedBy))
  ;[1 1 1] Server deals with health and damage stuff
  (bind _output_get (set `self.Health` (- (`self.Health`) Damage)))
  (if (<= _output_get 0.0)
    (`/Engine/EditorBlueprintResources/StandardMacros.DoOnce` false
      (:`Completed`
        (`/Engine/EditorBlueprintResources/StandardMacros.IsValid` InstigatedBy
          (:`Is Valid`
            (`/Engine/EditorBlueprintResources/StandardMacros.IsValid` _playerstate
              (:`Is Valid`
                (`/Engine/EditorBlueprintResources/StandardMacros.IsValid` (cast `/Game/TSS_Game/Blueprints/System/BP_PlayerState` _playerstate :!pure true)
                  (:`Is Valid`
                    _)
                  (:`Is Not Valid`
                    _)))
              (:`Is Not Valid`
                _)))
          (:`Is Not Valid`
            _))
        (set `self.isDead` true)
        (`MovementComponent.StopMovementImmediately` _charactermovement)
        (`NavMovementComponent.StopActiveMovement` _charactermovement)
        (`Controller.StopMovement` (`AIBlueprintHelperLibrary.GetAIController` self))
        (set `CharacterMovementComponent.MaxWalkSpeed` 0.0 _charactermovement)
        (`self.DetachFromControllerPendingDestroy` self)
        ;[1 1 1] Happens on all clients
        (`self.EnemyDeadMulticast`)))
    (else
      (`/Engine/EditorBlueprintResources/StandardMacros.IsValid` DamageCauser
        (:`Is Valid`
          (`self.MultiSpawnBlood` (`self.K2_GetActorLocation` DamageCauser)))))))

(event `MultiSpawnBlood`
  (params (Location :type "Vector Structure"))
  ;[1 1 1] Server deals with health and damage stuff
  (`GameplayStatics.SpawnEmitterAtLocation` "/Game/TSS_Game/Particles/P_body_bullet_impact.P_Body_Bullet_Impact" Location))

(fn `UserConstructionScript`)