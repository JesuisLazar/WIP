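; BP_Cube1 is a pickup cube labeled with its HealthName text, which destroys itself when a BP_CharacterBase overlaps it.
; On BeginPlay it sets the label and disables the cube's collision for three seconds before switching it to query-only.
; Tick forces the text to a fixed world rotation meant to face the camera.
; The overlap applies no health or other effect within this Blueprint.
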(event `self.ReceiveBeginPlay`
  (bind _cube (`self.Cube`))
  (`TextRenderComponent.K2_SetText` (`self.HealthName_TXT`) (`self.HealthName`))
  (`PrimitiveComponent.SetCollisionEnabled` _cube "NoCollision")
  (`KismetSystemLibrary.Delay` 3.0)
  (`PrimitiveComponent.SetCollisionEnabled` _cube "QueryOnly"))

(event `self.ReceiveTick`
  (params (DeltaSeconds :type "Float (single-precision)"))
  (`SceneComponent.K2_SetWorldRotation` (`self.HealthName_TXT`) (struct :`Pitch` 45.0 :`Yaw` 180.0) false false) ; Rotates the text to face the camera
)

(event `self.ReceiveActorBeginOverlap`
  (params (OtherActor :type "Actor Object Reference"))
  (cast `/Game/TSS_Game/Blueprints/System/BP_CharacterBase` OtherActor)
  (`self.K2_DestroyActor`))

(fn `UserConstructionScript`)