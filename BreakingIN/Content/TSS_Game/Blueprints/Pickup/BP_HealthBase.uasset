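; BP_HealthBase is a base health pickup that fully restores the health of a BP_CharacterBase that overlaps it.
; On overlap it casts to BP_CharacterBase, sets current health to maximum, then destroys itself.
; A text component shows the pickup's HealthName, set on BeginPlay.
; Tick reapplies a fixed world rotation to that text, meant to face the camera rather than tracking it dynamically.
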(event `self.ReceiveBeginPlay`
  (`TextRenderComponent.K2_SetText` (`self.HealthName_TXT`) (`self.HealthName`)))

(event `self.ReceiveTick`
  (params (DeltaSeconds :type "Float (single-precision)"))
  (`SceneComponent.K2_SetWorldRotation` (`self.HealthName_TXT`) (struct :`Pitch` 45.0 :`Yaw` 180.0) false false) ; Rotates the text to face the camera
)

(event `self.ReceiveActorBeginOverlap`
  (params (OtherActor :type "Actor Object Reference"))
  (bind _asbp_character_base (cast `/Game/TSS_Game/Blueprints/System/BP_CharacterBase` OtherActor))
  (set `/Game/TSS_Game/Blueprints/System/BP_CharacterBase.HealthCurrent` (`/Game/TSS_Game/Blueprints/System/BP_CharacterBase.HealthMax` _asbp_character_base) _asbp_character_base)
  (`self.K2_DestroyActor`))

(fn `UserConstructionScript`)