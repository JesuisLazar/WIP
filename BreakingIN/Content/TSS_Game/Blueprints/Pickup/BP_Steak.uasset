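; Steak pickup that advances an overlapping character's body-part completion.
; On spawn it launches its Cube with a mostly upward impulse and fills its floating label from HealthName.
; Tick holds the label at a fixed world rotation meant to face the camera.
; Overlap with a BP_CharacterBase whose PartOfBody is below three calls CheckBodyComplete on it and destroys the pickup; otherwise the steak remains.
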(event `self.ReceiveBeginPlay`
  ;[1 1 1] Set Text
  (`PrimitiveComponent.AddImpulse` (`self.Cube`) (50.0 50.0 10000.0) "None" false)
  (`TextRenderComponent.K2_SetText` (`self.HealthName_TXT`) (`self.HealthName`)))

(event `self.ReceiveTick`
  (params (DeltaSeconds :type "Float (single-precision)"))
  ;[1 1 1] Set Text
  ;;[1 1 1] Face rotation of the text
  (`SceneComponent.K2_SetWorldRotation` (`self.HealthName_TXT`) (struct :`Pitch` 45.0 :`Yaw` 180.0) false false) ; Rotates the text to face the camera
)

(event `self.ReceiveActorBeginOverlap`
  (params (OtherActor :type "Actor Object Reference"))
  ;[1 1 1] On overlap add or not part body
  (bind _asbp_character_base (cast `/Game/TSS_Game/Blueprints/System/BP_CharacterBase` OtherActor))
  (if (not (>= (`/Game/TSS_Game/Blueprints/System/BP_CharacterBase.PartOfBody` _asbp_character_base) 3))
    (`/Game/TSS_Game/Blueprints/System/BP_CharacterBase.CheckBodyComplete` _asbp_character_base)
    (`self.K2_DestroyActor`)))

(fn `UserConstructionScript`)