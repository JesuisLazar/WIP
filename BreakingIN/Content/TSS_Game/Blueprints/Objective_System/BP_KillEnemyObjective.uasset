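; Demo enemy character for the objective system that completes a GameMode objective when killed.
; It roams by repeatedly moving to random reachable navmesh points around itself with a short pause between moves.
; Damage lowers Health; at zero a DoOnce plays the death animation, ignores pawn collision and detaches the controller.
; It then completes a hardcoded objective entry and destroys itself after a delay.
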(event `self.ReceiveAnyDamage`
  (params (Damage :type "Float (single-precision)") (DamageType :type "DamageType Object Reference") (InstigatedBy :type "Controller Object Reference") (DamageCauser :type "Actor Object Reference"))
  ;[1 1 1] Demo Enemy
  (bind _output_get (set `self.Health` (- (`self.Health`) Damage)))
  (if (<= _output_get 0.0)
    ;[0.15 1 0] Objective system related
    (`/Engine/EditorBlueprintResources/StandardMacros.DoOnce` false ; Prevents from completing the same objective each time.
      (:`Completed`
        (`SkeletalMeshComponent.PlayAnimation` (`self.Mesh`) "/Game/TSS_Game/Character/AnimStarterPack/Death_1.Death_1" false)
        (`PrimitiveComponent.SetCollisionResponseToChannel` (`self.CapsuleComponent`) "ECC_Pawn" "ECR_Ignore")
        (`self.DetachFromControllerPendingDestroy`)
        (`/Game/TSS_Game/Blueprints/Objective_System/System/BPFL_Objectives.Complete_Objective` 1) ; Completes the specified entry inside the GameMode objectives array.
        (`KismetSystemLibrary.Delay` 5.0)
        (`self.K2_DestroyActor`)))))

(event `self.ReceiveBeginPlay`
  ;[1 1 1] Demo Enemy
  (`AITask_MoveTo.AIMoveTo` (`AIBlueprintHelperLibrary.GetAIController` self) (`NavigationSystemV1.K2_GetRandomReachablePointInRadius` (`self.K2_GetActorLocation`) 5000.0 null null) null :!label _label
    (:`OnMoveFinished`
      (`KismetSystemLibrary.Delay` 1.0)
      (goto _label))))

(fn `UserConstructionScript`)