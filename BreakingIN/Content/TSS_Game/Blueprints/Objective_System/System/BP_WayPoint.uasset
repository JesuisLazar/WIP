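; BP_WayPoint is an objective waypoint actor that shows its widget and minimap marker only while its assigned objective is current.
; On BeginPlay it caches the BP_GameModeObjectives game mode and starts a fast looping timer.
; Each timer call compares the game mode's CurrentObjectiveIndex with its own CurrentObjectiveActive, toggling widget visibility and adding or removing itself from the minimap, polling instead of reacting to objective-change events.
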(event `self.ReceiveBeginPlay`
  (bind _asbp_game_mode_objectives (cast `/Game/TSS_Game/Blueprints/Objective_System/System/BP_GameModeObjectives` (`GameplayStatics.GetGameMode`)))
  (set `self.GameModeCast` _asbp_game_mode_objectives)
  (`KismetSystemLibrary.K2_SetTimer` null "WayPointVisibility" 0.2 true))

(event `WayPointVisibility`
  (bind _gamemodecast (`self.GameModeCast`))
  (bind _returnvalue (== (`/Game/TSS_Game/Blueprints/Objective_System/System/BP_GameModeObjectives.CurrentObjectiveIndex` _gamemodecast) (`self.CurrentObjectiveActive`)))
  (`/Engine/EditorBlueprintResources/StandardMacros.IsValid` _gamemodecast
    (:`Is Valid`
      (`SceneComponent.SetVisibility` (`self.Widget`) _returnvalue false)
      (if _returnvalue
        (`/Game/TSS_Game/Blueprints/Objective_System/System/BPFL_Objectives.Minimap_Add` self)
        (else
          (`/Game/TSS_Game/Blueprints/Objective_System/System/BPFL_Objectives.Minimap_Remove` self))))))

(fn `UserConstructionScript`)