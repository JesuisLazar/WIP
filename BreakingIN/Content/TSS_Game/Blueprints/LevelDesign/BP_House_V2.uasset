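; BP_House_V2 is a level-design house actor that switches to its own fixed camera while a character is inside.
; On begin play it forces its spring arm to a fixed world rotation to prevent character movement glitches.
; An overlapping BP_CharacterBase hides the roof mesh, and its owning player controller blends view to the house.
; Leaving blends the view back to that character, and the roof reappears once no characters remain.
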(event `self.ReceiveBeginPlay`
  ;[1 1 1] Always sets camera to face world coordinates, prevents character movement glitches
  (`SceneComponent.K2_SetWorldRotation` (`self.SpringArm`) (struct :`Pitch` -90.0) false false))

(event `self.ReceiveActorBeginOverlap`
  (params (OtherActor :type "Actor Object Reference"))
  (bind _asbp_character_base (cast `/Game/TSS_Game/Blueprints/System/BP_CharacterBase` OtherActor))
  (`SceneComponent.SetVisibility` (`self.Mesh_Roof`) false false)
  (bind _owningplayercontroller (`/Game/TSS_Game/Blueprints/System/BP_CharacterBase.OwningPlayerController` _asbp_character_base))
  (`/Engine/EditorBlueprintResources/StandardMacros.IsValid` _owningplayercontroller
    (:`Is Valid`
      (`PlayerController.SetViewTargetWithBlend` _owningplayercontroller self 1.0 "VTBlend_Linear" 1.0 true))))

(event `self.ReceiveActorEndOverlap`
  (params (OtherActor :type "Actor Object Reference"))
  (bind _asbp_character_base (cast `/Game/TSS_Game/Blueprints/System/BP_CharacterBase` OtherActor))
  (if (not (> (`KismetArrayLibrary.Array_Length` (`self.GetOverlappingActors` "/Game/TSS_Game/Blueprints/System/BP_CharacterBase.BP_CharacterBase_C")) 0))
    (`SceneComponent.SetVisibility` (`self.Mesh_Roof`) true false))
  (bind _owningplayercontroller (`/Game/TSS_Game/Blueprints/System/BP_CharacterBase.OwningPlayerController` _asbp_character_base))
  (`/Engine/EditorBlueprintResources/StandardMacros.IsValid` _owningplayercontroller
    (:`Is Valid`
      (`PlayerController.SetViewTargetWithBlend` _owningplayercontroller _asbp_character_base 1.0 "VTBlend_Linear" 1.0 true))))

(fn `UserConstructionScript`)