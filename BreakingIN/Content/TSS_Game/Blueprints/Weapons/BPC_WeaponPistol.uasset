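; Pistol weapon Blueprint that adds firing animations to the Fire event of its parent weapon class.
; Fire runs the parent logic first, then checks that current ammo is above zero.
; If so, it plays the firing animation on the pistol mesh and a matching fire montage on the player's character mesh.
; BeginPlay and the construction script add no logic of their own.
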(event `self.Fire`
  (`parent.Fire`)
  (if (> (`self.AmmoCurrent`) 0)
    (`SkeletalMeshComponent.PlayAnimation` (`self.Pistol_Mesh`) "/Game/TSS_Game/Character/Weapons/Pistol/SK_Pistol_Auto_Skeleton_Firing.SK_Pistol_Auto_Skeleton_Firing" false)
    (`AnimInstance.Montage_Play` (`SkeletalMeshComponent.GetAnimInstance` (`Character.Mesh` (`self.PlayerCast`))) "/Game/TSS_Game/Character/AnimStarterPack/Fire_Pistol_Montage.Fire_Pistol_Montage" 1.0 "Duration" 0.0 true)))

(fn `UserConstructionScript`
  (`parent.UserConstructionScript`))