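; Base projectile actor for weapons that damages and pushes what it hits, then destroys itself.
; On hit it spawns an impact particle at the hit location and applies damage to the hit actor, credited to the instigator's controller.
; ApplyPhysics adds an impulse at the projectile's location to physics-simulating hit components, scaled from its velocity by a strength variable.
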(event `self.ReceiveHit`
  (params (MyComp :type "PrimitiveComponent Object Reference") (Other :type "Actor Object Reference") (OtherComp :type "PrimitiveComponent Object Reference") (bSelfMoved :type Boolean) (HitLocation :type "Vector Structure") (HitNormal :type "Vector Structure") (NormalImpulse :type "Vector Structure") (Hit :type "HitResult Structure (by ref)"))
  (`GameplayStatics.SpawnEmitterAtLocation` "/Game/TSS_Game/Particles/P_ImpactHit.P_ImpactHit" HitLocation)
  (`GameplayStatics.ApplyDamage` (`.HitActor` (`GameplayStatics.BreakHitResult` Hit)) (`self.ProjectileDamage`) (`self.GetInstigatorController` (`self.GetInstigator`)) self)
  (`self.ApplyPhysics` OtherComp)
  (`self.K2_DestroyActor`))

(fn `ApplyPhysics`
  (params (OtherComponent :type "PrimitiveComponent Object Reference"))
  (`/Engine/EditorBlueprintResources/StandardMacros.IsValid` OtherComponent
    (:`Is Valid`
      (if (`SceneComponent.IsSimulatingPhysics` OtherComponent "None")
        (`PrimitiveComponent.AddImpulseAtLocation` OtherComponent (* (`self.GetVelocity`) (`self.ProjectileImpulseStrenght`)) (`self.K2_GetActorLocation`) "None")
        (return)
        (else
          (return))))
    (:`Is Not Valid`
      (return))))

(fn `UserConstructionScript`)