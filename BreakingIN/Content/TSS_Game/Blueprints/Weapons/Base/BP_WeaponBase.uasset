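; Base weapon actor that serves as a named world pickup and, once equipped by a character, fires projectiles and reloads.
; Interaction adds and equips it, disables pickup collision, clears the label and plays the equip montage.
; Server-run Fire uses a DoOnce delay gate and looping timer for automatic fire, spending ammo, spawning projectiles from character or muzzle, then multicasting effects.
; Reload stops auto-fire and refills from reserve after its montage.
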(event `self.ReceiveTick`
  (params (DeltaSeconds :type "Float (single-precision)"))
  ;[1 1 1] Tick
  (if (not (`self.isTaken`))
    (`SceneComponent.K2_SetWorldRotation` (`self.WeaponNameText`) (struct :`Pitch` 45.0 :`Yaw` 180.0) false false) ; Rotates the text to face the camera
  ))

(event `self.ReceiveBeginPlay`
  (bind _weaponnametext (`self.WeaponNameText`))
  ;[1 1 1] Begin Play
  (set `self.SpawnedWeapon` self)
  (set `self.AmmoCurrent` (`self.AmmoMax`))
  (set `self.AmmoInReserveMax` (`self.AmmoInReserve`))
  (if (`self.isTaken`)
    (`TextRenderComponent.K2_SetText` _weaponnametext (`KismetTextLibrary.Conv_StringToText` " "))
    (else
      (`TextRenderComponent.K2_SetText` _weaponnametext (`self.WeaponName`)))))

(event `/Game/TSS_Game/Blueprints/System/BPI_Interactive.InteractWithWeapon`
  (params (CharacterReference :type "/Game/TSS_Game/Blueprints/System/BP_CharacterBase Object Reference"))
  ;[1 1 1] Equip
  (if (not (`self.isTaken`))
    (set `self.PlayerCast` CharacterReference)
    (`self.AddAndEquip` CharacterReference)))

(event `MultiPlayMontage`
  (bind _playercast (`self.PlayerCast`))
  ;[1 1 1] Equip
  (set `/Game/TSS_Game/Blueprints/System/BP_CharacterBase.isSwitchingWeapons` true _playercast)
  (bind _returnvalue (`AnimInstance.Montage_Play` (`SkeletalMeshComponent.GetAnimInstance` (`Character.Mesh` _playercast)) "/Game/TSS_Game/Character/AnimStarterPack/Equip_Rifle_Standing_Montage.Equip_Rifle_Standing_Montage" 2.0 "Duration" 0.0 true))
  (`KismetSystemLibrary.Delay` _returnvalue)
  (set `/Game/TSS_Game/Blueprints/System/BP_CharacterBase.isSwitchingWeapons` false _playercast))

(event `MulticastShowText`
  ;[1 1 1] Equip
  (`TextRenderComponent.K2_SetText` (`self.WeaponNameText`) (`KismetTextLibrary.Conv_StringToText` " ")))

(event `AddAndEquip`
  (params (CharacterReference :type "/Game/TSS_Game/Blueprints/System/BP_CharacterBase Object Reference"))
  ;[1 1 1] Equip
  (bind _indexoftheaddedweapon (`/Game/TSS_Game/Blueprints/System/BP_CharacterBase.AddWeapon` CharacterReference (`self.SpawnedWeapon`)))
  (`/Game/TSS_Game/Blueprints/System/BP_CharacterBase.EquipWeapon` CharacterReference _indexoftheaddedweapon)
  (`PrimitiveComponent.SetCollisionEnabled` (`self.Sphere`) "NoCollision")
  (set `self.isTaken` true)
  (`self.MulticastShowText`)
  (`self.MultiPlayMontage`))

(event `Fire`
  (bind _playercast (`self.PlayerCast`))
  (bind (_returnvalue_location _returnvalue_rotation) (`self.CalculateSpawnLocation` (`self.SpawnFromCharacter`)))
  ;[1 1 1] Fire - Runs on the Server (called from Character)
  (`/Engine/EditorBlueprintResources/StandardMacros.DoOnce` false :!label _label
    (:`Completed`
      (`|ExecutionSequence`
        (:`then_0`
          (if (`self.isReloading`)
            _
            (elif (`self.Automatic`)
              (`self.FireWeaponStarted`)
              (`KismetSystemLibrary.K2_SetTimer` null "FireWeaponStarted" (`self.Firerate`) true)
              (else
                (bind _canfire (`self.AmmoCheck` :!label _label_2))
                (if _canfire
                  (if (not (`/Game/TSS_Game/Blueprints/System/BP_CharacterBase.IsDead` (`self.PlayerCast`)))
                    (for _ (range (+ (`self.AdditionalProjectilesToFire`) 1))
                      (`|SpawnActorFromClass` (`self.ProjectileToFire`) (`KismetMathLibrary.MakeTransform` _returnvalue_location _returnvalue_rotation) "AlwaysSpawn" "OverrideRootScale" (`/Game/TSS_Game/Blueprints/System/BP_CharacterBase.OwningPlayerController` _playercast) (`self.Damage`) _playercast))
                    ;[1 1 1] Happens on all Clients
                    (`self.FireMulticastEvent`)))))))
        (:`then_1`
          (`KismetSystemLibrary.RetriggerableDelay` (`self.DelayBetweenShots`))
          (goto _label :!via `Reset`))))))

(event `FireWeaponStarted`
  ;[1 1 1] Fire - Runs on the Server (called from Character)
  (goto _label_2))

(event `FireMulticastEvent`
  ;[1 1 1] Happens on all Clients
  (`GameplayStatics.SpawnSoundAtLocation` (`self.FiringSound`) (`self.K2_GetActorLocation`) (struct) 1.0 1.0 0.0 null null) ; Firing Sound
  (`GameplayStatics.SpawnEmitterAttached` (`self.FiringEffect`) (`self.WeaponMesh`) (`self.MuzzleSocketName`) (0.0 0.0 0.0) (struct) (1.0 1.0 1.0) "SnapToTarget") ; Particle
)

(event `StopWeaponFire`
  ;[1 1 1] Fire - Runs on the Server (called from Character)
  (`KismetSystemLibrary.K2_ClearTimer` null "FireWeaponStarted"))

(event `Reload`
  ;[1 1 1] Reloading
  (`KismetSystemLibrary.K2_ClearTimer` null "FireWeaponStarted")
  (bind _canreload (`self.AmmoCheckMag`))
  (if _canreload
    (if (not (`self.isReloading`))
      (set `self.isReloading` true)
      (bind _returnvalue (`AnimInstance.Montage_Play` (`SkeletalMeshComponent.GetAnimInstance` (`Character.Mesh` (`self.PlayerCast`))) (`self.ReloadAnimMontage`) 1.0 "MontageLength" 0.0 true))
      (`KismetSystemLibrary.Delay` _returnvalue)
      (`self.AmmoReload`)
      (set `self.isReloading` false))))

(fn `AmmoCheck`
  (returns (CanFire :type Boolean))
  (if (> (`self.AmmoCurrent`) 0)
    (set `self.AmmoCurrent` (- (- (`self.AmmoCurrent`) 1) (`self.AdditionalProjectilesToFire`)))
    (return true)
    (else
      (return false))))

(fn `AmmoCheckMag`
  (returns (CanReload :type Boolean))
  (return (and (>= (`self.AmmoInReserve`) 1) (< (`self.AmmoCurrent`) (`self.AmmoMax`)))))

(fn `AmmoReload`
  (bind _zero (`self.Zero`))
  (bind _output_get (set `self.AmmoNeeded` (- (`self.AmmoMax`) (`self.AmmoCurrent`))))
  (`/Engine/EditorBlueprintResources/StandardMacros.CompareInt` (`self.AmmoInReserve`) (`self.AmmoMax`)
    (:`>`
      (set `self.AmmoCurrent` (`self.AmmoMax`) :!label _label))
    (:`==`
      (goto _label))
    (:`<`
      (set `self.AmmoCurrent` (`KismetMathLibrary.Clamp` (+ (`self.AmmoCurrent`) (`self.AmmoInReserve`)) (`self.Zero`) (`self.AmmoMax`)))))
  (bind _returnvalue (- (`self.AmmoInReserve`) _output_get))
  (`/Engine/EditorBlueprintResources/StandardMacros.CompareInt` _returnvalue _zero
    (:`>`
      (set `self.AmmoInReserve` _returnvalue))
    (:`==`
      (set `self.AmmoInReserve` _zero :!label _label_2))
    (:`<`
      (goto _label_2))))

(fn `CalculateSpawnLocation`
  (params (SpawnFromCharacter :type Boolean))
  (returns (ReturnValue_Location :type "Vector Structure") (ReturnValue_Rotation :type "Rotator Structure"))
  (bind _spread (`self.Spread`))
  (bind (_returnvalue_location _returnvalue_rotation) (`KismetMathLibrary.BreakTransform` (`SceneComponent.GetSocketTransform` (`self.WeaponMesh`) (`self.MuzzleSocketName`) "RTS_World")))
  (bind (_returnvalue_location_2 _returnvalue_rotation_2) (`KismetMathLibrary.BreakTransform` (`SceneComponent.K2_GetComponentToWorld` (`/Game/TSS_Game/Blueprints/System/BP_CharacterBase.BulletSpawnLocation` (`self.PlayerCast`)))))
  (bind (_returnvalue_roll _returnvalue_pitch _returnvalue_yaw) (`KismetMathLibrary.BreakRotator` (select `bool` SpawnFromCharacter :`false` _returnvalue_rotation :`true` _returnvalue_rotation_2)))
  (return (select `bool` SpawnFromCharacter :`false` _returnvalue_location :`true` _returnvalue_location_2) (`KismetMathLibrary.MakeRotator` _returnvalue_roll _returnvalue_pitch (select `bool` SpawnFromCharacter :`false` (+ _returnvalue_yaw (`KismetMathLibrary.RandomFloatInRange` (* _spread -1.0) _spread)) :`true` _returnvalue_yaw))))

(fn `UserConstructionScript`)