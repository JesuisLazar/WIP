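; Player controller for online and local co-op play, handling the possessed character link, UI widgets, kicking and logout.
; BeginPlay retries the character cast every second until it succeeds, then conditionally adds score and HUD widgets for local players.
; Coin helpers edit the PlayerState count, while update events refresh PlayerHUDWidget on remote local controllers.
; Tick feeds ammo, health and weapon name to PlayerHUD, whose creation code is unconnected here.
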(event `OnPlayerCoinCountUpdated`
  (params (PlayerID :type Integer))
  (`self.ForceNetUpdate`)
  (`/Engine/EditorBlueprintResources/ActorMacros.Switch Has Authority`
    (:`Remote`
      (if (`self.IsLocalPlayerController`)
        (`/Engine/EditorBlueprintResources/StandardMacros.IsValid` (`self.PlayerHUDWidget`)
          (:`Is Valid`
            (`/Game/TSS_Game/UI/WBP_PlayerHUD.UpdatePlayerCoinCount` (`self.PlayerHUDWidget`) PlayerID)))))))

(event `OnPlayersConnectionChanged`
  (`self.ForceNetUpdate`)
  (`/Engine/EditorBlueprintResources/ActorMacros.Switch Has Authority`
    (:`Remote`
      (if (`self.IsLocalPlayerController`)
        (`/Engine/EditorBlueprintResources/StandardMacros.IsValid` (`self.PlayerHUDWidget`)
          (:`Is Valid`
            (`/Game/TSS_Game/UI/WBP_PlayerHUD.UpdateActivePlayerList` (`self.PlayerHUDWidget`))))))))

(event `OnplayerControllerEnd`
  (bind _asbp_game_mode_base (cast `/Game/TSS_Game/Blueprints/System/BP_GameModeBase` (`GameplayStatics.GetGameMode`)))
  (`/Game/TSS_Game/Blueprints/System/BP_GameModeBase.OnPlayerLogout` _asbp_game_mode_base self))

(event `self.ReceiveEndPlay`
  (params (EndPlayReason :type "EEndPlayReason Enum" :default "Destroyed"))
  (`/Engine/EditorBlueprintResources/ActorMacros.Switch Has Authority`
    (:`Authority`
      (`self.OnplayerControllerEnd`))))

(event `TryAgainCast`
  (bind _asbp_character_base (cast `/Game/TSS_Game/Blueprints/System/BP_CharacterBase` (`self.K2_GetPawn`) :!label _label)
    (:`then`
      (bind _output_get (set `self.PlayerCast` _asbp_character_base))
      (set `/Game/TSS_Game/Blueprints/System/BP_CharacterBase.OwningPlayerController` self _output_get)
      (if (`self.IsLocalPlayerController`)
        (`/Engine/EditorBlueprintResources/StandardMacros.IsValid` (stale _returnvalue)
          (:`Is Not Valid`
            (bind _asbp_game_instance_with_settings (cast `/Game/TSS_Game/Blueprints/GameInstanceSettings/BP_GameInstanceWithSettings` (`GameplayStatics.GetGameInstance`)))
            (if (== (`/Game/TSS_Game/Blueprints/GameInstanceSettings/BP_GameInstanceWithSettings.LocalPlayers_Amount` _asbp_game_instance_with_settings) 0)
              (cast `/Game/TSS_Game/Blueprints/Objective_System/System/BP_GameModeObjectives` (`GameplayStatics.GetGameMode`)
                (:`CastFailed`
                  (bind _returnvalue (`|CreateWidget` "/Game/TSS_Game/UI/W_ScoreOnHUD.W_ScoreOnHUD_C" self))
                  (`UserWidget.AddToPlayerScreen` _returnvalue 0))))))))
    (:`CastFailed`
      (`KismetSystemLibrary.Delay` 1.0)
      (`self.TryAgainCast`))))

(event `self.ReceiveBeginPlay`
  (bind _playercast (`self.PlayerCast`))
  (`|ExecutionSequence`
    (:`then_0`
      (bind _asbp_game_instance_with_settings (cast `/Game/TSS_Game/Blueprints/GameInstanceSettings/BP_GameInstanceWithSettings` (`GameplayStatics.GetGameInstance`)))
      (bind _output_get (set `self.GameInstance_Cast` _asbp_game_instance_with_settings))
      (set `self.SelectedCharacter` (`/Game/TSS_Game/Blueprints/GameInstanceSettings/BP_GameInstanceWithSettings.SelectedCharacter` _output_get))
      (goto _label))
    (:`then_1`
      (`/Engine/EditorBlueprintResources/StandardMacros.IsValid` _playercast
        (:`Is Valid`
          (if (== (`GameplayStatics.GetPlayerControllerID` (`/Game/TSS_Game/Blueprints/System/BP_CharacterBase.OwningPlayerController` _playercast)) 0)
            (if (`self.IsLocalPlayerController`)
              (`|ExecutionSequence`
                (:`then_0`
                  (bind _returnvalue (`|CreateWidget` "/Game/TSS_Game/UI/WBP_PlayerHUD.WBP_PlayerHUD_C"))
                  (`UserWidget.AddToViewport` _returnvalue 0))))))))))

(event `ShowCountdown`
  (bind _returnvalue (`|CreateWidget` "/Game/BreakingIN/UI/W_countdown.W_countdown_C"))
  (`UserWidget.AddToViewport` _returnvalue 0))

(event `Showinfo`
  (bind _returnvalue (`|CreateWidget` "/Game/BreakingIN/UI/W_Info.W_Info_C"))
  (`UserWidget.AddToViewport` _returnvalue 0))

(event `Unfreeze`
  (`self.EnableInput` (`self.K2_GetPawn`) self))

(event `Key|U`
  (params (Key :type "Key Structure"))
  (:`Pressed`
    (bind _asbp_game_mode_base (cast `/Game/TSS_Game/Blueprints/System/BP_GameModeBase` (`GameplayStatics.GetGameMode`)))
    (`/Game/TSS_Game/Blueprints/System/BP_GameModeBase.Countdown` _asbp_game_mode_base)))

(event `InputAction|Pause`
  (params (Key :type "Key Structure"))
  (:`Pressed`
    (`/Engine/EditorBlueprintResources/StandardMacros.IsValid` (stale _returnvalue)
      (:`Is Not Valid`
        (bind _returnvalue (`|CreateWidget` "/Game/TSS_Game/UI/W_Disconnect.W_Disconnect_C" null self))
        (`UserWidget.AddToViewport` _returnvalue 0)))))

(event `Kick`
  (bind _gameinstance_cast (`self.GameInstance_Cast`))
  (if (`/Game/TSS_Game/Blueprints/GameInstanceSettings/BP_GameInstanceWithSettings.IsLocalCoopGame` _gameinstance_cast)
    (`GameplayStatics.RemovePlayer` self true)
    (set `/Game/TSS_Game/Blueprints/GameInstanceSettings/BP_GameInstanceWithSettings.LocalPlayers_Amount` (- (`/Game/TSS_Game/Blueprints/GameInstanceSettings/BP_GameInstanceWithSettings.LocalPlayers_Amount` _gameinstance_cast) 1) _gameinstance_cast)
    (else
      (`KismetSystemLibrary.ExecuteConsoleCommand` "disconnect" null))))

(event `self.ReceiveTick`
  (params (DeltaSeconds :type "Float (single-precision)"))
  (`self.UpdateHUD`))

(fn `Add Coin1`
  (bind _asbp_player_state (cast `/Game/TSS_Game/Blueprints/System/BP_PlayerState` (`self.PlayerState`)))
  (`/Engine/EditorBlueprintResources/StandardMacros.IncrementInt` (`/Game/TSS_Game/Blueprints/System/BP_PlayerState.PlayerCoin` _asbp_player_state)))

(fn `CompareControllerID`
  (params (ID :type Integer))
  (returns (True :type Boolean))
  (bind _playercast (`self.PlayerCast`))
  (`/Engine/EditorBlueprintResources/StandardMacros.IsValid` _playercast
    (:`Is Valid`
      (return (== (`GameplayStatics.GetPlayerControllerID` (`/Game/TSS_Game/Blueprints/System/BP_CharacterBase.OwningPlayerController` _playercast)) ID)))))

(fn `RemoveAllCoin1`
  (returns (TotalCoinDropped :type Integer))
  (bind _asbp_player_state (cast `/Game/TSS_Game/Blueprints/System/BP_PlayerState` (`self.PlayerState`)))
  (`|ExecutionSequence`
    (:`then_0`
      (set `self.CoinTotal` (`/Game/TSS_Game/Blueprints/System/BP_PlayerState.PlayerCoin` _asbp_player_state)))
    (:`then_1`
      (set `/Game/TSS_Game/Blueprints/System/BP_PlayerState.PlayerCoin` 0 _asbp_player_state))
    (:`then_2`
      (return (`self.CoinTotal`)))))

(fn `UpdateHUD`
  (bind _playercast (`self.PlayerCast`))
  (bind _playerhud (`self.PlayerHUD`))
  (bind _equippedweapon (`/Game/TSS_Game/Blueprints/System/BP_CharacterBase.EquippedWeapon` _playercast))
  (`/Engine/EditorBlueprintResources/StandardMacros.IsValid` _playercast
    (:`Is Valid`
      (`/Engine/EditorBlueprintResources/StandardMacros.IsValid` _equippedweapon
        (:`Is Valid`
          (`/Engine/EditorBlueprintResources/StandardMacros.IsValid` _playerhud
            (:`Is Valid`
              (`TextBlock.SetText` (`/Game/TSS_Game/UI/W_PlayerHUD.Ammo_TXT` _playerhud) (`KismetTextLibrary.Conv_StringToText` (`KismetStringLibrary.Concat_StrStr` (`KismetStringLibrary.Conv_IntToString` (`/Game/TSS_Game/Blueprints/Weapons/Base/BP_WeaponBase.AmmoCurrent` _equippedweapon)) "/" (`KismetStringLibrary.Conv_IntToString` (`/Game/TSS_Game/Blueprints/Weapons/Base/BP_WeaponBase.AmmoInReserve` _equippedweapon)))))
              (`ProgressBar.SetPercent` (`/Game/TSS_Game/UI/W_PlayerHUD.HealthBar` _playerhud) (`/Game/TSS_Game/Blueprints/System/BP_CharacterBase.HealthCurrent` _playercast))
              (`TextBlock.SetText` (`/Game/TSS_Game/UI/W_PlayerHUD.WeaponNameTXT` _playerhud) (`/Game/TSS_Game/Blueprints/Weapons/Base/BP_WeaponBase.WeaponName` _equippedweapon)))))))))

(fn `UserConstructionScript`)