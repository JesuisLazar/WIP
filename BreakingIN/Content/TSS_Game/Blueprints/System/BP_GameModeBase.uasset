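; Game mode that runs a timed multiplayer match with split-screen support and player kicking.
; PostLogin registers controllers and spawns their selected characters at PlayerStarts; BeginPlay adds local players from GameInstance settings and respawns existing pawns as a ServerTravel workaround.
; Countdown waits before unfreezing players and starting a looping timer that decrements GameState time until zero.
; Connection and coin-count changes are relayed to all player controllers.
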(event `Count`
  ;[1 1 1] Count + Timer
  (bind _result (`/Engine/EditorBlueprintResources/StandardMacros.DecrementInt` (`/Game/TSS_Game/Blueprints/System/BP_GameStateBase.CurrentTime` (`self.GameStateBase`)))
    (:`  `
      (if (== _result 0)
        (`KismetSystemLibrary.K2_PauseTimerHandle` (stale `Unfreeze` _returnvalue))))))

(event `Unfreeze`
  ;[1 1 1] Unfreeze
  (for _array_element (`self.Players`)
    (`/Game/TSS_Game/Blueprints/System/BP_PlayerController.Unfreeze` _array_element))
  ;[1 1 1] Count + Timer
  (set `/Game/TSS_Game/Blueprints/System/BP_GameStateBase.CurrentTime` (`self.matchTime`) (`self.GameStateBase`))
  (bind _returnvalue (`KismetSystemLibrary.K2_SetTimerDelegate` (delegate `Count`) 1.0 true))
  (`self.ShowTimers`))

(event `ShowTimers`
  ;[1 1 1] Count + Timer
  (for _array_element (`self.Players`)
    (`/Game/TSS_Game/Blueprints/System/BP_PlayerController.Showinfo` _array_element)))

(event `Countdown`
  ;[1 1 1] Countdown
  (if (not (`self.Started`))
    (for _array_element (`self.Players`)
      (`/Game/TSS_Game/Blueprints/System/BP_PlayerController.ShowCountdown` _array_element))
    (set `self.Started` true)
    (`KismetSystemLibrary.Delay` 3.0)
    (`self.Unfreeze`)))

(event `AddSplitScreenPlayer`
  (params (n :type Integer))
  ;[1 1 1] Split screen
  ;;[1 1 1] Create new local player for split screen
  (switch `int` n
    (:`1`
      (`GameplayStatics.CreatePlayer` -1))
    (:`2`
      (`GameplayStatics.CreatePlayer` -1)
      (`GameplayStatics.CreatePlayer` -1))
    (:`3`
      (`GameplayStatics.CreatePlayer` -1)
      (`GameplayStatics.CreatePlayer` -1)
      (`GameplayStatics.CreatePlayer` -1))))

(event `self.ReceiveBeginPlay`
  (`|ExecutionSequence`
    (:`then_0`
      ;[1 1 1] Split screen
      (bind _asbp_game_instance_with_settings (cast `/Game/TSS_Game/Blueprints/GameInstanceSettings/BP_GameInstanceWithSettings` (`GameplayStatics.GetGameInstance`)))
      (set `self.GameInstanceReference` _asbp_game_instance_with_settings)
      (bind _localplayers_amount (`/Game/TSS_Game/Blueprints/GameInstanceSettings/BP_GameInstanceWithSettings.LocalPlayers_Amount` _asbp_game_instance_with_settings))
      (if (not (== (`KismetArrayLibrary.Array_Length` (`GameStateBase.PlayerArray` (`GameplayStatics.GetGameState`))) (+ _localplayers_amount 1)))
        (`self.AddSplitScreenPlayer` _localplayers_amount)))
    (:`then_1`
      ;[1 1 1] ServerTravel workaround without making it in C++
      (for _array_element (`self.Players`)
        (bind _returnvalue (`Controller.K2_GetPawn` _array_element))
        (`/Engine/EditorBlueprintResources/StandardMacros.IsValid` _returnvalue
          (:`Is Valid`
            (`self.K2_DestroyActor` _returnvalue)
            (bind _outactors (`GameplayStatics.GetAllActorsOfClass` "/Script/Engine.PlayerStart"))
            (bind _asbp_player_controller (cast `/Game/TSS_Game/Blueprints/System/BP_PlayerController` _array_element :!pure true))
            (bind _returnvalue_2 (`|SpawnActorFromClass` (`/Game/TSS_Game/Blueprints/System/BP_PlayerController.SelectedCharacter` _asbp_player_controller) (`self.GetTransform` (`|GetArrayItem` _outactors)) "AlwaysSpawn" "OverrideRootScale" null "" null))
            (`Controller.Possess` _asbp_player_controller _returnvalue_2)
            (`/Game/TSS_Game/Blueprints/System/BP_PlayerController.TryAgainCast` _asbp_player_controller)
            (`self.RestartPlayer` _asbp_player_controller)))))
    (:`then_2`
      (bind _asbp_game_state_base (cast `/Game/TSS_Game/Blueprints/System/BP_GameStateBase` (`GameplayStatics.GetGameState`)))
      (set `self.GameStateBase` _asbp_game_state_base))))

(event `self.K2_PostLogin`
  (params (NewPlayer :type "PlayerController Object Reference"))
  (bind _returnvalue (`PlayerState.GetPlayerName` (`Controller.PlayerState` NewPlayer)))
  (bind _asbp_player_controller (cast `/Game/TSS_Game/Blueprints/System/BP_PlayerController` NewPlayer))
  (bind _returnvalue_2 (`KismetArrayLibrary.Array_Add` (`self.Players`) _asbp_player_controller))
  ;[1 1 1] Optional - spawns a custom character
  (bind _outactors (`GameplayStatics.GetAllActorsOfClass` "/Script/Engine.PlayerStart"))
  (bind _returnvalue_3 (`|SpawnActorFromClass` (`/Game/TSS_Game/Blueprints/System/BP_PlayerController.SelectedCharacter` _asbp_player_controller) (`self.GetTransform` (`|GetArrayItem` _outactors _returnvalue_2)) "AlwaysSpawn" "OverrideRootScale" null _returnvalue null))
  (set `/Game/TSS_Game/Blueprints/System/BP_CharacterBase.PlayerName` _returnvalue _returnvalue_3)
  (`Controller.Possess` NewPlayer _returnvalue_3)
  (`/Game/TSS_Game/Blueprints/System/BP_PlayerController.TryAgainCast` _asbp_player_controller)
  (`self.OnPlayerConnectionChanged`))

(event `KickPlayer`
  (params (PlayerID :type Integer))
  ;[1 1 1] Kicks a player (Press P/ESC to open the menu)
  (for (_array_element _array_index) (`self.Players`)
    (if (== _array_index PlayerID)
      (`/Engine/EditorBlueprintResources/StandardMacros.IsValid` _array_element
        (:`Is Valid`
          (bind _asbp_player_controller (cast `/Game/TSS_Game/Blueprints/System/BP_PlayerController` _array_element))
          (`/Game/TSS_Game/Blueprints/System/BP_PlayerController.Kick` _asbp_player_controller))))))

(event `OnPlayerConnectionChanged`
  (for _array_element (`self.Players`)
    (`/Engine/EditorBlueprintResources/StandardMacros.IsValid` _array_element
      (:`Is Valid`
        (`/Game/TSS_Game/Blueprints/System/BP_PlayerController.OnPlayersConnectionChanged` _array_element)))))

(event `OnPlayerCoinCountChanged`
  (params (PlayerID :type Integer))
  (for _array_element (`self.Players`)
    (`/Engine/EditorBlueprintResources/StandardMacros.IsValid` _array_element
      (:`Is Valid`
        (`/Game/TSS_Game/Blueprints/System/BP_PlayerController.OnPlayerCoinCountUpdated` _array_element PlayerID)))))

(event `OnPlayerLogout`
  (params (`Player Controller` :type "/Game/TSS_Game/Blueprints/System/BP_PlayerController Object Reference"))
  (`KismetArrayLibrary.Array_RemoveItem` (`self.Players`) `Player Controller`)
  (`self.OnPlayerConnectionChanged`))

(fn `UserConstructionScript`)